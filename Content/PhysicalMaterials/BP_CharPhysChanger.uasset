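; BP_CharPhysChanger is a surface actor that alters how the third-person character moves on it, making it slippery, grippy or bouncy.
; On overlap it optionally swaps the character's ground friction and walking braking deceleration, caching the originals to restore when overlap ends.
; Cube hits with a downward-facing normal launch the character vertically, reversing its last vertical velocity scaled by Bouncyness.
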(event OnComponentHit(Cube)
  (params (HitComponent :type Primitive%20Component%20Object%20Reference) (OtherActor :type Actor%20Object%20Reference) (OtherComp :type Primitive%20Component%20Object%20Reference) (NormalImpulse :type Vector :default "0, 0, 0") (Hit :type Hit%20Result%20Structure%20%28by%20ref%29))
  (if (<= (.z (.Normal (Collision|BreakHitResult Hit))) -0.5)
    (bind _asbp_third_person_character (Utilities|Casting|CastToBP_ThirdPersonCharacter OtherActor))
    (if (> (Variables|Default|GetBouncyness) 0.1)
      (Character|LaunchCharacter _asbp_third_person_character (Math|Vector|MakeVector 0.0 0.0 (* (.z (Pawn|Components|CharacterMovement|GetLastUpdateVelocity (Variables|/Script/Engine.Character|GetCharacterMovement _asbp_third_person_character))) -1.0 (Variables|Default|GetBouncyness))) false true))))

(event Collision|EventActorBeginOverlap
  (params (OtherActor :type Actor%20Object%20Reference))
  (bind _asbp_third_person_character (Utilities|Casting|CastToBP_ThirdPersonCharacter OtherActor))
  (if (Variables|Default|GetbChangeFriction)
    (Variables|Default|SetDefaultGroundFriction (Variables|/Script/Engine.CharacterMovementComponent|GetGroundFriction (Variables|/Script/Engine.Character|GetCharacterMovement _asbp_third_person_character)))
    (Variables|Default|SetDefaultBrakingDecelerationWalking (Variables|/Script/Engine.CharacterMovementComponent|GetBrakingDecelerationWalking (Variables|/Script/Engine.Character|GetCharacterMovement _asbp_third_person_character)))
    (Variables|/Script/Engine.CharacterMovementComponent|SetGroundFriction (Variables|/Script/Engine.Character|GetCharacterMovement _asbp_third_person_character) (Variables|Default|GetGround%20Friction))
    (Variables|/Script/Engine.CharacterMovementComponent|SetBrakingDecelerationWalking (Variables|/Script/Engine.Character|GetCharacterMovement _asbp_third_person_character) (Variables|Default|GetBraking%20Deceleration%20Walking))))

(event Collision|EventActorEndOverlap
  (params (OtherActor :type Actor%20Object%20Reference))
  (bind _asbp_third_person_character (Utilities|Casting|CastToBP_ThirdPersonCharacter OtherActor))
  (if (Variables|Default|GetbChangeFriction)
    (Variables|/Script/Engine.CharacterMovementComponent|SetGroundFriction (Variables|/Script/Engine.Character|GetCharacterMovement _asbp_third_person_character) (Variables|Default|GetDefaultGroundFriction))
    (Variables|/Script/Engine.CharacterMovementComponent|SetBrakingDecelerationWalking (Variables|/Script/Engine.Character|GetCharacterMovement _asbp_third_person_character) (Variables|Default|GetDefaultBrakingDecelerationWalking))))

(fn ConstructionScript)