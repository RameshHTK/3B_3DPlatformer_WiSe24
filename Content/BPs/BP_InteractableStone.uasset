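; BP_InteractableStone is a rune stone that switches its emissive glow on or off when interacted with.
; BeginPlay creates a dynamic material instance on the stone mesh.
; Each Interact event flips EmissionStrength by subtracting it from one and writes it to the material parameter of the same name.
; IsOn reports the stone's state by checking whether EmissionStrength equals one, so the glow value doubles as the state.
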(event EventBeginPlay
  (bind _returnvalue (Rendering|Material|CreateDynamicMaterialInstance (Variables|Default|GetSM_RuneStone_02) 0 0 "None" :!class /Script/Engine.PrimitiveComponent))
  (Variables|Default|SetMID _returnvalue))

(event EventInteract
  (bind _output_get (Variables|Default|SetEmissionStrength (- 1.0 (Variables|Default|GetEmissionStrength))))
  (Rendering|Material|SetScalarParameterValue (Variables|Default|GetMID) "EmissionStrength" _output_get :!class /Script/Engine.MaterialInstanceDynamic))

(fn ConstructionScript)

(fn Ison
  (return (== (Variables|Default|GetEmissionStrength) 1.0)))