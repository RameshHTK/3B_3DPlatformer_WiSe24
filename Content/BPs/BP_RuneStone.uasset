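; BP_RuneStone is an actor whose rune stone mesh glows, rises and spins as the player approaches.
; Each tick it converts player distance into an inverted, clamped 0-1 proximity value that reaches zero at 1000 units.
; That value drives emission on a dynamic material instance, float height and yaw speed, with spin squared for a sharper ramp and scaled by delta time.
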(event EventTick
  (params (DeltaSeconds :type Float%20%28single-precision%29))
  (bind _returnvalue (CallFunction|GetDistancetoPlayer))
  (bind _distance__0___1_ (CallFunction|Distanceto(0-1) _returnvalue))
  (CallFunction|SetMaterialEmission _distance__0___1_)
  (CallFunction|UpdateFloat _distance__0___1_)
  (CallFunction|Rotate _distance__0___1_))

(event EventBeginPlay
  (bind _returnvalue (Rendering|Material|CreateDynamicMaterialInstance (Variables|Default|GetRuneStone) 0 0 "None" :!class /Script/Engine.PrimitiveComponent))
  (Variables|Default|SetMID _returnvalue))

(fn ConstructionScript)

(fn GetDistancetoPlayer
  (return (Math|Vector|VectorLength (- (Transformation|GetActorLocation) (Transformation|GetActorLocation (Game|Player|GetPlayerPawn 0))))))

(fn Distanceto(0-1)
  (params (Distance :type Float%20%28double-precision%29))
  (return (- 1.0 (Math|Float|Clamp(Float) (/ Distance 1e+03)))))

(fn SetMaterialEmission
  (params (EmissionStrength :type Float%20%28single-precision%29))
  (Rendering|Material|SetScalarParameterValue (Variables|Default|GetMID) "EmissionStrength" EmissionStrength :!class /Script/Engine.MaterialInstanceDynamic))

(fn UpdateFloat
  (params (FloatAmount :type Float%20%28double-precision%29))
  (Transformation|SetRelativeLocation (Variables|Default|GetRuneStone) (Math|Vector|MakeVector 0.0 0.0 (* (Variables|Default|GetFloatHeight) FloatAmount)) false false))

(fn Rotate
  (params (Rotate%20Rate :type Float%20%28double-precision%29))
  (Transformation|AddRelativeRotation (Variables|Default|GetRuneStone) (Math|Rotator|MakeRotator 0.0 0.0 (* (* Rotate%20Rate Rotate%20Rate) (Variables|Default|GetMax%20RotationSpeed) (Utilities|Time|GetWorldDeltaSeconds))) false false))

(fn AddRotationF
  (params (RotationAmount :type Float%20%28double-precision%29))
  (Transformation|AddLocalRotation (Variables|Default|GetRuneStone) (Math|Rotator|MakeRotator 0.0 0.0 RotationAmount) false false)
  (return (.yaw (Variables|/Script/Engine.SceneComponent|GetRelativeRotation (Variables|Default|GetRuneStone)))))