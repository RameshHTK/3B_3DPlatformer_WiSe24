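; BP_Collectible is a pickup that spins in place until the third-person character overlaps it, then animates and destroys itself.
; Tick yaws the Pivot component at a constant idle speed, scaled by delta time.
; The first valid overlap passes a DoOnce into a timeline whose curves drive Pivot height, extra spin and uniform scale.
; When the timeline finishes the actor is destroyed, with no score or inventory update in this graph.
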(event Collision|EventActorBeginOverlap
  (params (OtherActor :type Actor%20Object%20Reference))
  (Utilities|Casting|CastToBP_ThirdPersonCharacter OtherActor)
  (Utilities|FlowControl|DoOnce false
    (:Completed
      (bind (_direction _zmovement _rotationspeed _size) (Timeline|Timeline Play)
        (:Update
          (Transformation|SetRelativeLocation (Variables|Default|GetPivot) (Math|Vector|MakeVector 0.0 0.0 (* _zmovement (Variables|Default|GetAnim_ZDist))) false false)
          (Transformation|AddRelativeRotation (Variables|Default|GetPivot) (Math|Rotator|MakeRotator 0.0 0.0 (* _rotationspeed (Variables|Default|GetAnim_RotSpeed) (Utilities|Time|GetWorldDeltaSeconds))) false false)
          (Transformation|SetWorldScale3D (Variables|Default|GetPivot) (* _size "1.000000,1.000000,1.000000")))
        (:Finished
          (Actor|DestroyActor))))))

(event EventTick
  (params (DeltaSeconds :type Float%20%28single-precision%29))
  (Transformation|AddRelativeRotation (Variables|Default|GetPivot) (Math|Rotator|MakeRotator 0.0 0.0 (* (Variables|Default|GetIdleRotSpeed) (Utilities|Time|GetWorldDeltaSeconds))) false false))

(fn ConstructionScript)