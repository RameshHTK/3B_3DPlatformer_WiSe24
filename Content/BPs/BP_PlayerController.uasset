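; Player controller that receives Enhanced Input and drives the possessed third-person character.
; It adds the third-person mapping context on BeginPlay and caches the character reference on possession.
; Input actions forward jump, yaw-only camera rotation and movement to that character.
; Movement feeds the input axes straight into world X and Y, so it is not relative to the camera.
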(event Input|EnhancedActionEvents|EnhancedInputActionIA_RotateCamera
  (params (ActionValue :type Float%20%28double-precision%29) (ElapsedSeconds :type Float%20%28double-precision%29) (TriggeredSeconds :type Float%20%28double-precision%29) (InputAction :type Input%20Action%20Object%20Reference :default "/Game/Input/InputActions/IA_RotateCamera.IA_RotateCamera"))
  (Pawn|Input|AddControllerYawInput (Variables|Default|GetPossessed%20Third%20Person%20Character) ActionValue))

(event Input|EnhancedActionEvents|EnhancedInputActionIA_Jump
  (params (ActionValue :type Boolean) (ElapsedSeconds :type Float%20%28double-precision%29) (TriggeredSeconds :type Float%20%28double-precision%29) (InputAction :type Input%20Action%20Object%20Reference :default "/Game/Input/InputActions/IA_Jump.IA_Jump"))
  (Character|Jump (Variables|Default|GetPossessed%20Third%20Person%20Character)))

(event Input|EnhancedActionEvents|EnhancedInputActionIA_Move
  (params (ActionValue :type Vector%202D%20Structure) (ElapsedSeconds :type Float%20%28double-precision%29) (TriggeredSeconds :type Float%20%28double-precision%29) (InputAction :type Input%20Action%20Object%20Reference :default "/Game/Input/InputActions/IA_Move.IA_Move"))
  (Pawn|Input|AddMovementInput (Variables|Default|GetPossessed%20Third%20Person%20Character) (Math|Vector|MakeVector (.x ActionValue) (.y ActionValue) 0.0) 1.0 false))

(event EventBeginPlay
  (Input|AddMappingContext (PlayerController|LocalPlayerSubsystems|GetEnhancedInputLocalPlayerSubsystem) "/Game/Input/IMC_ThirdPerson.IMC_ThirdPerson" 0 "(bIgnoreAllPressedKeysUntilRelease=True,bForceImmediately=False,bNotifyUserSettings=False)"))

(event EventPossess
  (params (PossessedPawn :type Pawn%20Object%20Reference))
  (bind _asbp_third_person_character (Utilities|Casting|CastToBP_ThirdPersonCharacter PossessedPawn))
  (Variables|Default|SetPossessed%20Third%20Person%20Character _asbp_third_person_character))

(fn ConstructionScript)