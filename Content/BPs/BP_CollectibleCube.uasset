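; BP_CollectibleCube is a collectible cube pickup that reports its collection to the player's UI.
; OnCollected calls OnCollectedCube on the ThirdPersonCharacter's CollectibleWidget.
; PlayCollectAnimation plays a timeline that drives the uniform scale of the Pivot component, then destroys the actor when it finishes.
; Tick and the construction script only call the parent, and nothing in this graph triggers either collection event.
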(event EventPlayCollectAnimation
  (bind _scale (Timeline|Anim Play)
    (:Update
      (Transformation|SetRelativeScale3D (Variables|Default|GetPivot) (* "1.000000,1.000000,1.000000" _scale)))
    (:Finished
      (Actor|DestroyActor))))

(event EventTick
  (params (DeltaSeconds :type Float%20%28single-precision%29))
  (|CallParentFunction DeltaSeconds))

(event EventOnCollected
  (params (ThirdPersonCharacter :type BP%20Third%20Person%20Character%20Object%20Reference))
  (Default|OnCollectedCube (Variables|/Game/BPs/BP_ThirdPersonCharacter.BP_ThirdPersonCharacter_C|GetCollectibleWidget ThirdPersonCharacter)))

(fn ConstructionScript
  (|CallParentFunction))