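; BP_SplinePlatform is a platform actor that moves continuously along the spline of an assigned SplineActor.
; On BeginPlay it prints an on-screen error if no spline actor is set, otherwise it plays a timeline that restarts whenever it finishes.
; Each update scales the timeline's percentage by spline length to get a world-space transform, setting location without sweep and, if AlignToSpline is enabled, rotation.
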(event Custom|MoveAlongSpline
  (bind _splinepercentage (Timeline|Timeline PlayFromStart)
    (:Update
      (Transformation|SetActorLocation (.Location (CallFunction|GetLocationandRotationfromSpline _splinepercentage)) false false)
      (if (Variables|Default|GetbAlignToSpline)
        (Transformation|SetActorRotation (.Rotation (CallFunction|GetLocationandRotationfromSpline _splinepercentage)))))
    (:Finished
      (CallFunction|MoveAlongSpline))))

(event EventBeginPlay
  ;[1 1 1] BeginPlay
  (Utilities|IsValid (Variables|Default|GetSplineActor)
    (:Is%20Valid
      (CallFunction|MoveAlongSpline))
    (:Is%20Not%20Valid
      (Development|PrintString "SplinePlatform: Spline actor is not assigned!" true true "(R=1.000000,G=0.053995,B=0.000000,A=1.000000)" 1e+01))))

(fn ConstructionScript)

(fn GetLocationandRotationfromSpline
  (params (DistanceAlongSpline%20%25 :type Float%20%28double-precision%29))
  (bind _splineactor (Variables|Default|GetSplineActor))
  (bind _spline (Variables|/Game/BPs/Plarforms/BP_SplineActor.BP_SplineActor_C|GetSpline _splineactor))
  (bind _returnvalue (Spline|GetSplineLength _spline))
  (bind _returnvalue_2 (* DistanceAlongSpline%20%25 _returnvalue))
  (return (Spline|GetLocationatDistanceAlongSpline _spline _returnvalue_2 "World") (Spline|GetRotationatDistanceAlongSpline _spline _returnvalue_2 "World")))